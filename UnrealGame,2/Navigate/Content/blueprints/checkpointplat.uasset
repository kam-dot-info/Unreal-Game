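; Checkpoint platform that restores the player's health to maximum and moves the respawn point when its trigger is overlapped.
; Begin overlap updates player health, plays the platform animation, sound and Niagara effect, teleports the first SpawnPos actor to the Spawnlocation component, and shows text until overlap ends.
; It uses player character 0 without checking the overlapping actor, and re-fires on every overlap.
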(event `self.trigger.OnComponentBeginOverlap`
  (params (OverlappedComponent :type "PrimitiveComponent Object Reference") (OtherActor :type "Actor Object Reference") (OtherComp :type "PrimitiveComponent Object Reference") (OtherBodyIndex :type Integer) (bFromSweep :type Boolean) (SweepResult :type "HitResult Structure (by ref)"))
  (bind (_returnvalue_location _returnvalue_rotation) (`KismetMathLibrary.BreakTransform` (`SceneComponent.K2_GetComponentToWorld` (`self.spawnlocation`))))
  (bind _asbp_third_person_character (cast `/Game/ThirdPerson/Blueprints/BP_ThirdPersonCharacter` (`GameplayStatics.GetPlayerCharacter` 0)))
  (bind _output_get (set `self.As BP Third Person Character` _asbp_third_person_character))
  (bind _output_get_2 (set `/Game/ThirdPerson/Blueprints/BP_ThirdPersonCharacter.Health` (`/Game/ThirdPerson/Blueprints/BP_ThirdPersonCharacter.Maxhealth` _output_get) _output_get))
  (`/Game/ThirdPerson/Blueprints/BP_ThirdPersonCharacter.ED-UpdateHealth` (`self.As BP Third Person Character`) _output_get_2)
  (`SkeletalMeshComponent.PlayAnimation` (`self.platform`) "/Game/mesh/checkpointplat/chechpoint_Anim.chechpoint_Anim" false)
  (`GameplayStatics.PlaySound2D` "/Game/sounds/checkpointsound.checkpointsound" 1.0 1.0 0.0 null null)
  (`ActorComponent.Activate` (`self.Paricle-NS`) false)
  (bind _outactors (`GameplayStatics.GetAllActorsOfClass` "/Game/blueprints/SpawnPos.SpawnPos_C"))
  (`self.K2_SetActorTransform` (`|GetArrayItem` _outactors) (`KismetMathLibrary.MakeTransform` _returnvalue_location _returnvalue_rotation) false true)
  (`SceneComponent.SetVisibility` (`self.TextRender`) true false))

(event `self.trigger.OnComponentEndOverlap`
  (params (OverlappedComponent :type "PrimitiveComponent Object Reference") (OtherActor :type "Actor Object Reference") (OtherComp :type "PrimitiveComponent Object Reference") (OtherBodyIndex :type Integer))
  (`SceneComponent.SetVisibility` (`self.TextRender`) false false))

(fn `UserConstructionScript`)