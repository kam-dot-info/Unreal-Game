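; Spike trap actor that damages the third-person player who steps into its collision volume, on a cooldown.
; Overlap plays the spike animation and sound, then a short delay gives the player a window to escape.
; Any end-overlap during that window sets a dodge flag that cancels the damage.
; A Cooldown timeline blocks retriggering until it finishes.
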(event `self.Collision.OnComponentBeginOverlap`
  (params (OverlappedComponent :type "PrimitiveComponent Object Reference") (OtherActor :type "Actor Object Reference") (OtherComp :type "PrimitiveComponent Object Reference") (OtherBodyIndex :type Integer) (bFromSweep :type Boolean) (SweepResult :type "HitResult Structure (by ref)"))
  (set `self.DodgeCheck` false)
  ;[1 1 1] Casting
  (bind _asbp_third_person_character (cast `/Game/ThirdPerson/Blueprints/BP_ThirdPersonCharacter` OtherActor))
  (set `self.As BP Third Person Character` _asbp_third_person_character)
  ;[1 1 1] Cooldown Check
  (if (not (`self.CooldownCheck`))
    (set `self.CooldownCheck` true) ; sets cooldown before running code
    ;[1 1 1] Sound and Anim
    (`SkeletalMeshComponent.PlayAnimation` (`self.spikes`) "/Game/mesh/spiketraps/spikes/spikespikes_Anim.spikespikes_Anim" false)
    (`GameplayStatics.PlaySound2D` "/Game/sounds/spikesfx.spikesfx" 1.0 1.0 0.0 null null)
    ;[1 1 1] Dodge check
    (`KismetSystemLibrary.Delay` 0.75) ; time user takes to dodge
    (if (`self.DodgeCheck`)
      (set `self.DodgeCheck` false)
      ;[1 1 1] Cooldown
      (`Timeline|Cooldown` :!label _label ; 3.5s timer, once finished cooldown is reset
        (:`Finished`
          (set `self.CooldownCheck` false)))
      (else
        ;[1 1 1] damage
        (`GameplayStatics.ApplyDamage` (`self.As BP Third Person Character`) 40.0)
        (set `self.DodgeCheck` false)
        (goto _label)))))

(event `self.Collision.OnComponentEndOverlap`
  (params (OverlappedComponent :type "PrimitiveComponent Object Reference") (OtherActor :type "Actor Object Reference") (OtherComp :type "PrimitiveComponent Object Reference") (OtherBodyIndex :type Integer))
  (set `self.DodgeCheck` true))

(fn `UserConstructionScript`)