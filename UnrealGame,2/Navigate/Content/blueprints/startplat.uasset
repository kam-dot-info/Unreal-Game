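; Starting platform actor whose Startplat mesh animates in response to a Box trigger volume.
; BeginPlay plays Homestart_Anim once without looping.
; Entering the Box plays the animation forward and leaving plays it in reverse by flipping the play rate, with no filter on the overlapping actor.
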(event `self.ReceiveBeginPlay`
  ;[1 1 1] play anim
  (`SkeletalMeshComponent.PlayAnimation` (`self.startplat`) "/Game/mesh/start/home-start_Anim.home-start_Anim" false))

(event `self.Box.OnComponentEndOverlap`
  (params (OverlappedComponent :type "PrimitiveComponent Object Reference") (OtherActor :type "Actor Object Reference") (OtherComp :type "PrimitiveComponent Object Reference") (OtherBodyIndex :type Integer))
  ;[1 1 1] reverse
  (`SkeletalMeshComponent.SetPlayRate` (`self.startplat`) -1.0)
  (`SkeletalMeshComponent.Play` (`self.startplat`) false))

(event `self.Box.OnComponentBeginOverlap`
  (params (OverlappedComponent :type "PrimitiveComponent Object Reference") (OtherActor :type "Actor Object Reference") (OtherComp :type "PrimitiveComponent Object Reference") (OtherBodyIndex :type Integer) (bFromSweep :type Boolean) (SweepResult :type "HitResult Structure (by ref)"))
  (`SkeletalMeshComponent.SetPlayRate` (`self.startplat`) 1.0)
  (`SkeletalMeshComponent.Play` (`self.startplat`) false))

(fn `UserConstructionScript`)