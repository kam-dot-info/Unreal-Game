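; Health pickup actor that restores health to the player's third-person character when touched.
; On begin play it loops an animation on its mesh.
; A box overlap casts player character 0, adds a fixed amount to its Health without clamping, broadcasts the UpdateHealth dispatcher for the UI, then destroys itself.
; The overlapping actor is never checked, so any overlap heals the player.
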(event `self.ReceiveBeginPlay`
  ;[1 1 1] health
  (`SkeletalMeshComponent.PlayAnimation` (`self.class-healpowerup`) "/Game/mesh/health/class-healpowerup_Anim.class-healpowerup_Anim" true))

(event `self.Box.OnComponentBeginOverlap`
  (params (OverlappedComponent :type "PrimitiveComponent Object Reference") (OtherActor :type "Actor Object Reference") (OtherComp :type "PrimitiveComponent Object Reference") (OtherBodyIndex :type Integer) (bFromSweep :type Boolean) (SweepResult :type "HitResult Structure (by ref)"))
  ;[1 1 1] Casting
  (bind _asbp_third_person_character (cast `/Game/ThirdPerson/Blueprints/BP_ThirdPersonCharacter` (`GameplayStatics.GetPlayerCharacter` 0)))
  (set `self.As BP Third Person Character` _asbp_third_person_character)
  ;[0.298 0.8196 0.2157] Add Health
  (bind _output_get (set `/Game/ThirdPerson/Blueprints/BP_ThirdPersonCharacter.Health` (+ 40.0 (`/Game/ThirdPerson/Blueprints/BP_ThirdPersonCharacter.Health` (`self.As BP Third Person Character`))) (`self.As BP Third Person Character`))) ; setting health
  (`/Game/ThirdPerson/Blueprints/BP_ThirdPersonCharacter.ED-UpdateHealth` (`self.As BP Third Person Character`) _output_get) ; updating health to ui
  (`self.K2_DestroyActor`))

(fn `UserConstructionScript`)