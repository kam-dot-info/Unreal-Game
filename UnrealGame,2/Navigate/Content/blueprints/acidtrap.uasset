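; Acid trap hazard that damages the player character, with a looping puddle animation started on BeginPlay.
; Overlapping the Col collision plays a sound and starts a Timeline that applies fixed damage on every update, using it as a damage ticker.
; Ending the overlap stops the Timeline.
; The overlap always targets player 0's BP_ThirdPersonCharacter, without checking which actor entered or left.
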(event `self.ReceiveBeginPlay`
  (`SkeletalMeshComponent.PlayAnimation` (`self.puddle`) "/Game/mesh/acid/acidpuddle_Anim.acidpuddle_Anim" true))

(event `self.col.OnComponentBeginOverlap`
  (params (OverlappedComponent :type "PrimitiveComponent Object Reference") (OtherActor :type "Actor Object Reference") (OtherComp :type "PrimitiveComponent Object Reference") (OtherBodyIndex :type Integer) (bFromSweep :type Boolean) (SweepResult :type "HitResult Structure (by ref)"))
  (bind _asbp_third_person_character (cast `/Game/ThirdPerson/Blueprints/BP_ThirdPersonCharacter` (`GameplayStatics.GetPlayerCharacter` 0)))
  (set `self.As BP Third Person Character` _asbp_third_person_character)
  (`GameplayStatics.PlaySound2D` "/Game/sounds/acidsfx.acidsfx" 1.0 1.0 0.0 null null)
  (`Timeline|Timeline` :!label _label
    (:`tick`
      (`GameplayStatics.ApplyDamage` (`self.As BP Third Person Character`) 4.0))))

(event `self.col.OnComponentEndOverlap`
  (params (OverlappedComponent :type "PrimitiveComponent Object Reference") (OtherActor :type "Actor Object Reference") (OtherComp :type "PrimitiveComponent Object Reference") (OtherBodyIndex :type Integer))
  (goto _label :!via `Stop`))

(fn `UserConstructionScript`)