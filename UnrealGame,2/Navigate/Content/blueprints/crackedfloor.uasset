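; A cracked floor actor that falls away shortly after the third-person character touches it, then gets respawned.
; On overlap with its collision, it waits briefly, enables physics simulation on the floor mesh, then disables it a few seconds later.
; It passes the transform saved at BeginPlay to the game mode's RespawnCrackedFloor and destroys itself, leaving replacement to the game mode.
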(event `self.ReceiveBeginPlay`
  (set `self.StartingLocation` (`SceneComponent.K2_GetComponentToWorld` (`self.DefaultSceneRoot`))))

(event `self.collision.OnComponentBeginOverlap`
  (params (OverlappedComponent :type "PrimitiveComponent Object Reference") (OtherActor :type "Actor Object Reference") (OtherComp :type "PrimitiveComponent Object Reference") (OtherBodyIndex :type Integer) (bFromSweep :type Boolean) (SweepResult :type "HitResult Structure (by ref)"))
  (cast `/Game/ThirdPerson/Blueprints/BP_ThirdPersonCharacter` OtherActor)
  (`KismetSystemLibrary.Delay` 0.2)
  (`PrimitiveComponent.SetSimulatePhysics` (`self.floor`) true)
  (`KismetSystemLibrary.Delay` 3.0)
  (`PrimitiveComponent.SetSimulatePhysics` (`self.floor`) false)
  (bind _asbp_third_person_game_mode (cast `/Game/ThirdPerson/Blueprints/BP_ThirdPersonGameMode` (`GameplayStatics.GetGameMode`)))
  (`/Game/ThirdPerson/Blueprints/BP_ThirdPersonGameMode.RespawnCrackedFloor` _asbp_third_person_game_mode (`self.StartingLocation`))
  (`self.K2_DestroyActor`))

(fn `UserConstructionScript`)