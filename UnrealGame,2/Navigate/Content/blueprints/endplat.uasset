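; End platform actor that closes out the game when something overlaps its end collision.
; That overlap plays an end-game sound, starts the ending level sequence through a newly created player, then quits after a short fixed delay.
; A separate light trigger switches the point light to high intensity on overlap and back to zero on exit.
; None of the overlap events filter which actor triggers them.
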(event `self.endcollision.OnComponentBeginOverlap`
  (params (OverlappedComponent :type "PrimitiveComponent Object Reference") (OtherActor :type "Actor Object Reference") (OtherComp :type "PrimitiveComponent Object Reference") (OtherBodyIndex :type Integer) (bFromSweep :type Boolean) (SweepResult :type "HitResult Structure (by ref)"))
  (`GameplayStatics.PlaySound2D` "/Game/sounds/endgamesound.endgamesound" 1.0 1.0 0.0 null null)
  (bind _outactor (`LevelSequencePlayer.CreateLevelSequencePlayer` "/Game/Sequences/EndingSeq.EndingSeq"))
  (`MovieSceneSequencePlayer.Play` (`LevelSequenceActor.SequencePlayer` _outactor))
  (`KismetSystemLibrary.Delay` 3.0)
  (`KismetSystemLibrary.QuitGame` null "Quit"))

(event `self.light trigger.OnComponentBeginOverlap`
  (params (OverlappedComponent :type "PrimitiveComponent Object Reference") (OtherActor :type "Actor Object Reference") (OtherComp :type "PrimitiveComponent Object Reference") (OtherBodyIndex :type Integer) (bFromSweep :type Boolean) (SweepResult :type "HitResult Structure (by ref)"))
  ;[1 1 1] LightSwitch
  (`LightComponent.SetIntensity` (`self.PointLight`) 100000.0))

(event `self.light trigger.OnComponentEndOverlap`
  (params (OverlappedComponent :type "PrimitiveComponent Object Reference") (OtherActor :type "Actor Object Reference") (OtherComp :type "PrimitiveComponent Object Reference") (OtherBodyIndex :type Integer))
  ;[1 1 1] LightSwitch
  (`LightComponent.SetIntensity` (`self.PointLight`) 0.0))

(fn `UserConstructionScript`)