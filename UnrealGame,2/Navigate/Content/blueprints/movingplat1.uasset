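; Moving platform Blueprint that starts a Timeline when anything begins overlapping its Box.
; Each Timeline update lerps the Cube's relative location from zero to EndLocation, then enters a five-second Delay.
; After the delay, EndLocation2 serves as both the character's world teleport target and the Cube's relative location.
; The cast that would set the character reference is disconnected, so this graph never assigns it.
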(event `self.Box.OnComponentBeginOverlap`
  (params (OverlappedComponent :type "PrimitiveComponent Object Reference") (OtherActor :type "Actor Object Reference") (OtherComp :type "PrimitiveComponent Object Reference") (OtherBodyIndex :type Integer) (bFromSweep :type Boolean) (SweepResult :type "HitResult Structure (by ref)"))
  (bind _end_location_2 (`self.End Location 2`))
  (bind (_direction _timemove) (`Timeline|Timeline`)
    (:`Update`
      (`SceneComponent.K2_SetRelativeLocation` (`self.Cube`) (`KismetMathLibrary.VLerp` (0.0 0.0 0.0) (`self.EndLocation`) _timemove) false false)
      (`KismetSystemLibrary.Delay` 5.0)
      (`self.K2_SetActorLocation` (`self.As BP Third Person Character`) _end_location_2 false true)
      (`SceneComponent.K2_SetRelativeLocation` (`self.Cube`) _end_location_2 false false))))

(fn `UserConstructionScript`)