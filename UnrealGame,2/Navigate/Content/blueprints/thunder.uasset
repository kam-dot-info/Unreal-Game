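; Thunder hazard that kills the player when something overlaps its collision.
; Any overlap fetches player 0's character, starts a looping thunder animation and plays a 2D sound.
; A small untargeted damage call for a powerup death check precedes, by a short delay, damage equal to the player's max health.
; A Timeline is meant as a cooldown, but CooldownCheck is only ever set false, so it never blocks retriggering.
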(event `self.collision.OnComponentBeginOverlap`
  (params (OverlappedComponent :type "PrimitiveComponent Object Reference") (OtherActor :type "Actor Object Reference") (OtherComp :type "PrimitiveComponent Object Reference") (OtherBodyIndex :type Integer) (bFromSweep :type Boolean) (SweepResult :type "HitResult Structure (by ref)"))
  (bind _as_bp_third_person_character (`self.As BP Third Person Character`))
  ;[1 1 1] Casting
  (bind _asbp_third_person_character (cast `/Game/ThirdPerson/Blueprints/BP_ThirdPersonCharacter` (`GameplayStatics.GetPlayerCharacter` 0)))
  (set `self.As BP Third Person Character` _asbp_third_person_character)
  ;[1 1 1] Cooldown Check
  (if (not (`self.Cooldown Check`))
    (set `self.Cooldown Check` false)
    ;[1 1 1] Sound and Anim
    (`SkeletalMeshComponent.PlayAnimation` (`self.thunder`) "/Game/mesh/thunder/thunder_Anim.thunder_Anim" true)
    (`GameplayStatics.PlaySound2D` "/Game/sounds/thundersfx.thundersfx" 1.0 1.0 0.0 null null)
    ;[1 1 1] damage
    (`GameplayStatics.ApplyDamage` null 0.1) ; for powerup death check
    (`KismetSystemLibrary.Delay` 0.1)
    (`GameplayStatics.ApplyDamage` _as_bp_third_person_character (`/Game/ThirdPerson/Blueprints/BP_ThirdPersonCharacter.Maxhealth` _as_bp_third_person_character))
    ;[1 1 1] Cooldown
    (`Timeline|Timeline` ; 3.5s timer, once finished cooldown is reset
      (:`Finished`
        (set `self.Cooldown Check` false)))))

(fn `UserConstructionScript`)